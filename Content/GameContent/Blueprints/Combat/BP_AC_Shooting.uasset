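; Shooting component that supplies hitscan aiming and tracing, aimed through the first player's camera.
; Source and direction come from player controller 0's camera manager, falling back to the owner's eye location and the parent class's direction when that controller is invalid.
; Hitscan extends that ray by FireDistance and line-traces against world static, world dynamic and one custom object type, returning the hit result.
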(fn `GetHitscanDirection`
  (returns (ReturnValue :type "Vector Structure"))
  (`/Engine/EditorBlueprintResources/StandardMacros.IsValid` (`GameplayStatics.GetPlayerController` 0)
    (:`Is Valid`
      (return (`KismetMathLibrary.GetForwardVector` (`PlayerCameraManager.GetCameraRotation` (`PlayerController.PlayerCameraManager` (`GameplayStatics.GetPlayerController` 0))))))
    (:`Is Not Valid`
      (return (`parent.GetHitscanDirection`)))))

(fn `GetHitscanSourceLocation`
  (returns (ReturnValue :type "Vector Structure"))
  (`/Engine/EditorBlueprintResources/StandardMacros.IsValid` (`GameplayStatics.GetPlayerController` 0)
    (:`Is Valid`
      (return (`PlayerCameraManager.GetCameraLocation` (`PlayerController.PlayerCameraManager` (`GameplayStatics.GetPlayerController` 0)))))
    (:`Is Not Valid`
      (return (`Actor.GetActorEyesViewPoint` (`self.GetOwner`))))))

(fn `Hitscan`
  (returns (Hit :type "HitResult Structure") (ReturnValue :type Boolean))
  (locals (L_Start :type "Vector Structure") (L_End :type "Vector Structure" :default (0.0 0.0 0.0)))
  (set `local.L_Start` (`self.GetHitscanSourceLocation`))
  (set `local.L_End` (+ (* (`self.GetHitscanDirection`) (`self.FireDistance`)) (`local.L_Start`)))
  (bind (_outhit _returnvalue) (`KismetSystemLibrary.LineTraceSingleForObjects` (`local.L_Start`) (`local.L_End`) (`|MakeArray` "ObjectTypeQuery8" "ObjectTypeQuery1" "ObjectTypeQuery2" :!type "EObjectTypeQuery Enum")))
  (return _outhit _returnvalue))